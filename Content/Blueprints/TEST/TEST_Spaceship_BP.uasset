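; Test spaceship pawn with Enhanced Input controls for forward thrust, yaw rotation and a fire action that only spawns an explosion emitter at the bullet socket.
; Tick wraps the ship horizontally by projecting its position to screen space and deprojecting the opposite edge.
; BeginPlay also prototypes off-ship spawning: after a delay it places a dummy actor at a random left-edge point with a debug line and explosion.
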(event Input|EnhancedActionEvents|EnhancedInputActionIA_Move
  (params (ActionValue :type Boolean) (ElapsedSeconds :type Float%20%28double-precision%29) (TriggeredSeconds :type Float%20%28double-precision%29) (InputAction :type Input%20Action%20Object%20Reference :default "/Game/Input/IA_Move.IA_Move"))
  (:Triggered
    (Class|PawnMovementComponent|AddInputVector (Variables|Default|GetFloatingPawnMovement) (Math|Vector|GetForwardVector (Variables|Default|GetSphere)) false)))

(event Input|EnhancedActionEvents|EnhancedInputActionIA_RotateShip
  (params (ActionValue :type Float%20%28double-precision%29) (ElapsedSeconds :type Float%20%28double-precision%29) (TriggeredSeconds :type Float%20%28double-precision%29) (InputAction :type Input%20Action%20Object%20Reference :default "/Game/Input/IA_RotateShip.IA_RotateShip"))
  (:Triggered
    (Transformation|AddWorldRotation (Variables|Default|GetSphere) (Math|Rotator|MakeRotator 0.0 0.0 (* (Variables|Default|GetRotSpeed) ActionValue (Utilities|Time|GetWorldDeltaSeconds))) false false)))

(event Input|EnhancedActionEvents|EnhancedInputActionIA_Fire
  (params (ActionValue :type Boolean) (ElapsedSeconds :type Float%20%28double-precision%29) (TriggeredSeconds :type Float%20%28double-precision%29) (InputAction :type Input%20Action%20Object%20Reference :default "/Game/Input/IA_Fire.IA_Fire"))
  (:Started
    (Effects|SpawnEmitteratLocation "/Game/StarterContent/Particles/P_Explosion.P_Explosion" (Transformation|GetSocketLocation (Variables|Default|GetStaticMesh) "BulletSpawnLoc"))))

(event EventBeginPlay
  (bind _returnvalue (Game|GetPlayerController 0))
  (Input|AddMappingContext (PlayerController|LocalPlayerSubsystems|GetEnhancedInputLocalPlayerSubsystem (Game|GetPlayerController 0)) "/Game/Input/Spaceship_IMC.Spaceship_IMC" 0 "(bIgnoreAllPressedKeysUntilRelease=True,bForceImmediately=False)")
  (Utilities|FlowControl|Delay 1.0)
  (bind _returnvalue_2 (Game|SpawnActorfromClass "/Game/Blueprints/TEST/DummActor_BP.DummActor_BP_C" (Math|Transform|MakeTransform (.WorldPosition (Class|GameplayStatics|DeprojectScreentoWorld _returnvalue (Math|Vector2D|MakeVector2D (Math|Random|RandomFloatinRange 0.0 0.0) (Math|Random|RandomFloatinRange 0.0 (Math|Conversions|ToFloat(Integer) (+ (.SizeY (HUD|GetViewportSize _returnvalue)) 50)))))) "0, 0, 0" "1.000000,1.000000,1.000000") "Undefined" 0 0))
  (Rendering|Debug|DrawDebugLine (.location (Transformation|GetActorTransform _returnvalue_2)) (Math|Vector|RotateVectorAroundAxis (- "" (.location (Transformation|GetActorTransform _returnvalue_2))) (Math|Random|RandomFloatinRange 9e+01 -9e+01) "0.000000,0.000000,1.000000") "(R=1.000000,G=1.000000,B=1.000000,A=1.000000)" 1e+01 0.0)
  (Effects|SpawnEmitteratLocation "/Game/StarterContent/Particles/P_Explosion.P_Explosion" (.location (Transformation|GetActorTransform _returnvalue_2))))

(event Collision|EventActorBeginOverlap
  (params (OtherActor :type Actor%20Object%20Reference)))

(event EventTick
  (params (DeltaSeconds :type Float%20%28single-precision%29))
  (bind _returnvalue (Game|GetPlayerController 0))
  (bind _returnvalue_2 (Transformation|GetActorLocation))
  (bind _returnvalue_3 (Transformation|GetActorLocation))
  (bind _screenposition (Class|GameplayStatics|ProjectWorldtoScreen _returnvalue _returnvalue_2 false))
  (bind (_sizex _sizey) (HUD|GetViewportSize _returnvalue))
  (bind (_x _y) (Math|Vector2D|BreakVector2D _screenposition))
  (Utilities|FlowControl|Sequence
    (:then_0
      (if (< _x 0.0)
        (Transformation|SetActorLocation (Math|Vector|MakeVector (.x _returnvalue_3) (.Y (Math|Vector|BreakVector (.WorldPosition (Class|GameplayStatics|DeprojectScreentoWorld _returnvalue (Math|Vector2D|MakeVector2D (Math|Conversions|ToFloat(Integer) _sizex) (Math|Conversions|ToFloat(Integer) _sizey)))))) 0.0) false false)))
    (:then_1
      (if (> _x _sizex)
        (Transformation|SetActorLocation (Math|Vector|MakeVector (.x _returnvalue_3) (.Y (Math|Vector|BreakVector (.WorldPosition (Class|GameplayStatics|DeprojectScreentoWorld _returnvalue (Math|Vector2D|MakeVector2D 0.0 _y))))) 0.0) false false)))))

(fn ConstructionScript)